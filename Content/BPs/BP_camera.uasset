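; Camera actor that travels point to point along the spline of a BP_PathCamera found in the level, wrapping to the first point after the last.
; Each tick it traces from the player camera along the view, biased against travel direction.
; A horizontal dot product of travel direction and pawn-to-hit vector raises or lowers speed within limits.
; Movement is an unswept world offset per frame, not scaled by delta time.
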(event EventBeginPlay
  (bind _returnvalue (Actor|GetActorOfClass "/Game/BPs/BP_PathCamera.BP_PathCamera_C"))
  (Variables|Default|SetPath _returnvalue))

(event EventTick
  (params (DeltaSeconds :type Float%20%28single-precision%29))
  (bind _returnvalue (Transformation|GetActorLocation))
  (bind _returnvalue_2 (Game|Player|GetPlayerPawn 0))
  (bind _returnvalue_3 (Game|GetPlayerCameraManager 0))
  (bind _returnvalue_4 (Transformation|GetActorLocation _returnvalue_2))
  (bind _returnvalue_5 (Camera|GetCameraLocation _returnvalue_3))
  (Variables|Default|SetDelta%20Seconds DeltaSeconds)
  (Variables|Default|SetCameraDirection (Math|Vector|Normalize (- (Spline|GetLocationatSplinePoint (Variables|/Game/BPs/BP_PathCamera.BP_PathCamera_C|GetSpline (Variables|Default|GetPath)) (Variables|Default|GetPoint%20Index) "World") _returnvalue)))
  (bind _outhit (Collision|LineTraceByChannel _returnvalue_5 (+ (- _returnvalue_5 (* (Variables|Default|GetCameraDirection) 2e+04)) (* (Math|Vector|GetForwardVector (Camera|GetCameraRotation _returnvalue_3)) 1e+05)) "TraceTypeQuery3" false 0 "None"))
  (Variables|Default|SetHitLocation (.location _outhit))
  (if (< (Math|Vector|Distance(Vector) (Spline|GetLocationatSplinePoint (Variables|/Game/BPs/BP_PathCamera.BP_PathCamera_C|GetSpline (Variables|Default|GetPath)) (Variables|Default|GetPoint%20Index) "World") _returnvalue) 5e+02)
    (if (>= (- (Spline|GetNumberOfSplinePoints (Variables|/Game/BPs/BP_PathCamera.BP_PathCamera_C|GetSpline (Variables|Default|GetPath))) 1) (Variables|Default|GetPoint%20Index))
      (Variables|Default|SetPoint%20Index (+ (Variables|Default|GetPoint%20Index) 1))
      (else
        (Variables|Default|SetPoint%20Index 0))))
  (if (<= (Math|Vector|DotProduct (Math|Vector|MakeVector (.x (Variables|Default|GetCameraDirection)) (.y (Variables|Default|GetCameraDirection)) 0.0) (- (Math|Vector|MakeVector (.x (Variables|Default|GetHitLocation)) (.y (Variables|Default|GetHitLocation)) 0.0) (Math|Vector|MakeVector (.x _returnvalue_4) (.y _returnvalue_4) 0.0))) 0.0)
    (if (< (Variables|Default|GetCameraSpeed) (Variables|Default|GetMaxCameraSpeed))
      (Variables|Default|SetCameraSpeed (+ (Variables|Default|GetCameraSpeed) (* (Variables|Default|GetDelta%20Seconds) 1e+01))))
    (elif (> (Variables|Default|GetCameraSpeed) (Variables|Default|GetMinCameraSpeed))
      (Variables|Default|SetCameraSpeed (- (Variables|Default|GetCameraSpeed) (* (Variables|Default|GetDelta%20Seconds) 1e+01)))))
  (Transformation|AddActorWorldOffset (* (Variables|Default|GetCameraDirection) (Variables|Default|GetCameraSpeed))))

(fn ConstructionScript)