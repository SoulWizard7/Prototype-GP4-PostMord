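; BP_Fence is a wooden fence that falls over when a BP_BoxTruck_Chaos drives into it.
; The Cube's overlap calls HitWoodFence on the truck, then snaps the Scene component to a 90 or 270 degree roll based on which side in world Y the truck is on.
; A DoOnce precedes the cast, so the first overlap by any actor uses up the trigger.
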(event OnComponentBeginOverlap(Cube)
  (params (OverlappedComponent :type Primitive%20Component%20Object%20Reference) (OtherActor :type Actor%20Object%20Reference) (OtherComp :type Primitive%20Component%20Object%20Reference) (OtherBodyIndex :type Integer) (bFromSweep :type Boolean) (SweepResult :type Hit%20Result%20Structure%20%28by%20ref%29))
  (bind _returnvalue (Transformation|GetActorRotation))
  (bind _scene (Variables|Default|GetScene))
  (Utilities|FlowControl|DoOnce false
    (:Completed
      (bind _asbp_box_truck_chaos (Utilities|Casting|CastToBP_BoxTruck_Chaos OtherActor))
      (Default|HitWoodFence _asbp_box_truck_chaos)
      (if (< (.y (Transformation|GetActorLocation OtherActor)) (.y (Transformation|GetActorLocation)))
        (Transformation|SetWorldRotation _scene (Math|Rotator|MakeRotator 9e+01 (.pitch _returnvalue) (.yaw _returnvalue)) false false)
        (else
          (Transformation|SetWorldRotation _scene (Math|Rotator|MakeRotator 2.7e+02 (.pitch _returnvalue) (.yaw _returnvalue)) false false))))))

(event EventBeginPlay)

(event Collision|EventActorBeginOverlap
  (params (OtherActor :type Actor%20Object%20Reference)))

(event EventTick
  (params (DeltaSeconds :type Float%20%28single-precision%29)))

(fn ConstructionScript)