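; BP_MailBox is a mailbox actor that catches overlapping actors tagged "paper".
; On overlap it turns off physics simulation on the paper's primitive component and teleports the paper to the location of its Cube1 component.
; It then spawns the NS_PaperBang Niagara effect at the NiagaraPosition component's transform.
; A node that would set the paper's root mobility to Stationary is left unconnected.
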(event EventBeginPlay)

(event Collision|EventActorBeginOverlap
  (params (OtherActor :type Actor%20Object%20Reference))
  (bind _niagaraposition (Variables|Default|GetNiagaraPosition))
  (bind _returnvalue (Transformation|GetWorldTransform _niagaraposition))
  (if (Actor|ActorHasTag OtherActor "paper")
    (Physics|SetSimulatePhysics (Actor|GetComponentbyClass OtherActor "/Script/Engine.PrimitiveComponent") false)
    (Transformation|SetActorLocation OtherActor (Transformation|GetWorldLocation (Variables|Default|GetCube1)) false true)
    (Niagara|SpawnSystematLocation "/Game/BPs/NS_PaperBang.NS_PaperBang" (.location _returnvalue) (.rotation _returnvalue))))

(event EventTick
  (params (DeltaSeconds :type Float%20%28single-precision%29)))

(fn ConstructionScript)