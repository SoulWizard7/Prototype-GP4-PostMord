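; Player controller for a truck-based mail-throwing game, viewed through a separately spawned BP_camera with the mouse cursor shown.
; A left-mouse drag records two height-flattened cursor hit points and passes them to the truck's ThrowMail.
; P destroys the truck and respawns one at a camera-based line trace hit, facing the camera's CameraDirection.
; The new truck is possessed and launched forward with an impulse, and the camera's speed is set.
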(event Custom|NewVehicle
  (bind _returnvalue (Game|GetPlayerCameraManager 0))
  (bind _returnvalue_2 (Camera|GetCameraLocation _returnvalue))
  (bind _outhit (Collision|LineTraceByChannel _returnvalue_2 (+ (- _returnvalue_2 (* (Variables|/Game/BPs/BP_camera.BP_camera_C|GetCameraDirection (Variables|Default|GetCamera%20Actor)) 8e+04)) (* (Math|Vector|GetForwardVector (Camera|GetCameraRotation _returnvalue)) 1e+05)) "TraceTypeQuery3" false 0 "ForOneFrame"))
  (bind _returnvalue_3 (Game|SpawnActorfromClass "/Game/VehicleVarietyVol2/Blueprints/BoxTruck/BP_BoxTruck_Chaos.BP_BoxTruck_Chaos_C" (Math|Transform|MakeTransform (.location _outhit) (Math|Conversions|RotationFromXVector (Variables|/Game/BPs/BP_camera.BP_camera_C|GetCameraDirection (Variables|Default|GetCamera%20Actor))) "1.000000,1.000000,1.000000") "AdjustIfPossibleButAlwaysSpawn" 0 0))
  (Pawn|Possess _returnvalue_3)
  (Variables|Default|SetVehicle _returnvalue_3)
  (Game|Player|SetViewTargetwithBlend (Variables|Default|GetCamera%20Actor) 0.0 "VTBlend_Linear" 0.0 false)
  (Physics|AddImpulse (Variables|/Script/ChaosVehicles.WheeledVehiclePawn|GetMesh (Variables|Default|GetVehicle)) (* (Transformation|GetActorForwardVector (Variables|Default|GetVehicle)) 4e+06) "None" false)
  (Variables|/Game/BPs/BP_camera.BP_camera_C|SetCameraSpeed (Variables|Default|GetCamera%20Actor) 0.5))

(event EventBeginPlay
  (bind _spawn_transform (Variables|Default|GetSpawn%20Transform))
  (bind _asbp_box_truck_chaos (Utilities|Casting|CastToBP_BoxTruck_Chaos (Game|Player|GetPlayerPawn 0)))
  (Variables|Default|SetVehicle _asbp_box_truck_chaos)
  (Development|PrintString "cast worked")
  (Variables|Default|SetbShowMouseCursor true)
  (bind _returnvalue (Game|SpawnActorfromClass "/Game/BPs/BP_camera.BP_camera_C" (Math|Transform|MakeTransform (+ (.location (Transformation|GetActorTransform (Game|Player|GetPlayerPawn 0))) (.location _spawn_transform)) (.rotation _spawn_transform) "1.000000,1.000000,1.000000") "Undefined" 0 0))
  (bind _output_get (Variables|Default|SetCamera%20Actor _returnvalue))
  (Game|Player|SetViewTargetwithBlend _output_get 2.0 "VTBlend_Linear" 0.0 false))

(event EventTick
  (params (DeltaSeconds :type Float%20%28single-precision%29)))

(event Input|MouseEvents|LeftMouseButton
  (params (Key :type Key%20Structure :default "None"))
  (bind _hitresult (Game|Player|GetHitResultUnderCursorbyChannel "TraceTypeQuery3" true))
  (:Pressed
    (bind _output_get (Variables|Default|SetHit%20Result%20Impact%20Point (.impactpoint _hitresult)))
    (Variables|Default|SetMousePos1 (Math|Vector|MakeVector (.x _output_get) (.y _output_get) 0.0)))
  (:Released
    (bind _output_get_2 (Variables|Default|SetHit%20Result%20Impact%20Point (.impactpoint _hitresult)))
    (Variables|Default|SetMousePos2 (Math|Vector|MakeVector (.x _output_get_2) (.y _output_get_2) 0.0))
    (Default|ThrowMail (Variables|Default|GetVehicle) (Variables|Default|GetMousePos1) (Variables|Default|GetMousePos2))))

(event Input|KeyboardEvents|P
  (params (Key :type Key%20Structure :default "None"))
  (:Pressed
    (Default|DestroyVehicle (Variables|Default|GetVehicle))
    (CallFunction|NewVehicle)))

(fn ConstructionScript)