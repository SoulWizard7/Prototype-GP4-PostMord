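; Drivable Chaos box truck pawn that throws paper mail.
; Axis input drives steering, camera and handbrake, but throttle is forced full below a speed threshold and braking works only above another, keeping the truck moving.
; ThrowMail launches a spawned BP_Paper along a given direction with lift and spin, while bush and fence hits trigger Niagara effects.
; Tipping over requests a new vehicle from BP_PlayerController, then destroys the truck after a delay, as does DestroyVehicle.
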(event Custom|ThrowMail
  (params (Pos1 :type Vector) (Pos2 :type Vector))
  (bind _returnvalue (Game|SpawnActorfromClass "/Game/BPs/BP_Paper.BP_Paper_C" (Transformation|GetWorldTransform (Variables|Default|GetPaperSpawnTransform)) "Undefined" 0 0))
  (Physics|AddForce (Variables|/Game/BPs/BP_Paper.BP_Paper_C|GetCube _returnvalue) (* (Math|Vector|Normalize (- Pos2 Pos1)) (Variables|Default|GetPaper%20Throw%20Force)) "None" false)
  (Physics|AddForce (Variables|/Game/BPs/BP_Paper.BP_Paper_C|GetCube _returnvalue) "0, 0,100000.000000" "None" false)
  (Class|PrimitiveComponent|AddTorqueinRadians (Variables|/Game/BPs/BP_Paper.BP_Paper_C|GetCube _returnvalue) "0.000000,0.000000,1000.000000" "None" true))

(event Custom|HitBush
  (Components|Activation|Activate (Variables|Default|GetNiagara) true))

(event Custom|HitWoodFence
  (Components|Activation|Activate (Variables|Default|GetNiagara1) true))

(event Custom|Destroy%20Vehicle
  (Utilities|FlowControl|Delay 5.0)
  (Actor|DestroyActor))

(event EventTick
  (params (DeltaSeconds :type Float%20%28single-precision%29))
  (if (< (Math|Vector|DotProduct (Transformation|GetActorUpVector) (Math|Vector|VectorUp)) 0.1)
    (Utilities|FlowControl|DoOnce false
      (:Completed
        (bind _asbp_player_controller (Utilities|Casting|CastToBP_PlayerController (Game|GetPlayerController 0)))
        (Default|NewVehicle _asbp_player_controller)
        (Utilities|FlowControl|Delay 5.0)
        (Actor|DestroyActor)))))

(event Input|ActionEvents|InputActionHandbrake
  (params (Key :type Key%20Structure :default "None"))
  (bind _vehiclemovementcomponent (Variables|Default|GetVehicleMovementComponent))
  (:Pressed
    (Class|ChaosVehicleMovementComponent|SetHandbrakeInput _vehiclemovementcomponent true)
    (Variables|Default|SetIs%20Handbrake%20on? true))
  (:Released
    (Class|ChaosVehicleMovementComponent|SetHandbrakeInput _vehiclemovementcomponent false)
    (Variables|Default|SetIs%20Handbrake%20on? false)))

(event Input|AxisEvents|InputAxisMoveRight
  (params (AxisValue :type Float%20%28single-precision%29))
  (Class|ChaosVehicleMovementComponent|SetSteeringInput (Variables|Default|GetVehicleMovementComponent) AxisValue))

(event Input|AxisEvents|InputAxisTurn
  (params (AxisValue :type Float%20%28single-precision%29))
  (Pawn|Input|AddControllerYawInput AxisValue))

(event Input|AxisEvents|InputAxisLookUp
  (params (AxisValue :type Float%20%28single-precision%29))
  (Pawn|Input|AddControllerPitchInput AxisValue))

(event Input|AxisEvents|InputAxisMoveForward
  (params (AxisValue :type Float%20%28single-precision%29))
  (if (< (Vehicle|GetForwardSpeed (Variables|Default|GetVehicleMovementComponent)) 8e+02)
    (Class|ChaosVehicleMovementComponent|SetThrottleInput (Variables|Default|GetVehicleMovementComponent) 1.0)
    (else
      (Class|ChaosVehicleMovementComponent|SetThrottleInput (Variables|Default|GetVehicleMovementComponent) AxisValue))))

(event Input|AxisEvents|InputAxisReverse/Brake
  (params (AxisValue :type Float%20%28single-precision%29))
  (if (> (Vehicle|GetForwardSpeed (Variables|Default|GetVehicleMovementComponent)) 7e+02)
    (Class|ChaosVehicleMovementComponent|SetBrakeInput (Variables|Default|GetVehicleMovementComponent) AxisValue)
    (else
      (Class|ChaosVehicleMovementComponent|SetBrakeInput (Variables|Default|GetVehicleMovementComponent) 0.0))))

(fn ConstructionScript)